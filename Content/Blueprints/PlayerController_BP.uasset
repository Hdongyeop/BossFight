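; Player controller Blueprint that holds back the local player's look and move input until the game starts.
; On BeginPlay it binds to the OnGameStarted dispatcher on the Manager game instance, then, for a local controller, shows the mouse cursor and ignores look and move input.
; When the dispatcher fires, it re-enables both inputs but leaves the cursor setting unchanged.
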(event Custom|OnGameStarted_Event
  (Input|SetIgnoreLookInput false)
  (Input|SetIgnoreMoveInput false))

(event EventBeginPlay
  (bind _asmanager (Utilities|Casting|CastToManager (Game|GetGameInstance)))
  (EventDispatchers|AssignOnGameStarted _asmanager (delegate Custom|OnGameStarted_Event))
  (if (Pawn|IsLocalPlayerController)
    (Variables|Default|SetbShowMouseCursor true)
    (Input|SetIgnoreLookInput true)
    (Input|SetIgnoreMoveInput true)))

(event EventTick
  (params (DeltaSeconds :type Float%20%28single-precision%29)))

(fn ConstructionScript)