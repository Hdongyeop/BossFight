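; Base enemy Blueprint, initialized with Boss stats, that targets and attacks playable characters.
; SphereVision overlaps set or clear the AI blackboard Target; Tick, gated by GameStarted, drops dead targets.
; ATK_01 and ATK_02 face the target and play random montages, with ATK_02 also timeline-lerping toward player 0 until close.
; DoDamage sphere-overlaps at DamageArrow, applying StatComponent damage to living playable characters.
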(event OnComponentBeginOverlap(SphereVision)
  (params (OverlappedComponent :type Primitive%20Component%20Object%20Reference) (OtherActor :type Actor%20Object%20Reference) (OtherComp :type Primitive%20Component%20Object%20Reference) (OtherBodyIndex :type Integer) (bFromSweep :type Boolean) (SweepResult :type Hit%20Result%20Structure%20%28by%20ref%29))
  ;[0.3854 0.3854 0.3854] Overlap Set, Get and Clear Target
  (if (!= OtherActor self)
    (bind _asplayable_character (Utilities|Casting|CastToPlayableCharacter OtherActor))
    (CallFunction|SetTarget _asplayable_character)))

(event OnComponentEndOverlap(SphereVision)
  (params (OverlappedComponent :type Primitive%20Component%20Object%20Reference) (OtherActor :type Actor%20Object%20Reference) (OtherComp :type Primitive%20Component%20Object%20Reference) (OtherBodyIndex :type Integer))
  ;[0.3854 0.3854 0.3854] Overlap Set, Get and Clear Target
  (if (== OtherActor (CallFunction|GetTarget))
    (CallFunction|ClearTarget)))

(event Custom|ATK_02
  (params (Target :type Actor%20Object%20Reference))
  ;[0.4522 0.4522 0.4522] ATK_02(Air Attack)
  (Utilities|FlowControl|Sequence
    (:then_0
      (Utilities|IsValid Target
        (:Is%20Valid
          (bind _returnvalue (Transformation|SetActorRotation (Math|Rotator|MakeRotator 0.0 0.0 (.yaw (Math|Rotator|FindLookatRotation (Transformation|GetActorLocation) (Transformation|GetActorLocation Target)))))))))
    (:then_1
      (Animation|PlayAnimMontage (Utilities|Array|Get(acopy) (Variables|Default|GetAttackArray) (Math|Random|RandomIntegerinRange 2 3)) 1.0 "None"))
    (:then_2
      (bind _alpha (Timeline|Alpha%280~1%29 PlayFromStart)
        (:Update
          (if (> 1e+02 (Transformation|GetDistanceTo (Game|GetPlayerCharacter 0)))
            (Audio|Components|Audio|Stop (Variables|Default|GetAlpha%280~1%29))
            (else
              (Transformation|SetActorLocation (Math|Vector|Lerp(Vector) (Transformation|GetActorLocation) (Transformation|GetActorLocation (Game|GetPlayerCharacter 0)) _alpha) false false))))))))

(event Custom|DoDamage
  ;[0.3385 0.3385 0.3385] DoDamage
  (bind (_outactors _returnvalue) (Collision|SphereOverlapActors (Transformation|GetWorldLocation (Variables|Default|GetDamageArrow)) (Variables|Default|GetDamageRadius) (Utilities|Array|MakeArray "ObjectTypeQuery3") 0 (Utilities|Array|MakeArray self)))
  (if _returnvalue
    (for _array_element _outactors
      (bind _asplayable_character (Utilities|Casting|CastToPlayableCharacter _array_element))
      (if (not (<= (Variables|/Script/BossFight.StatComponent|GetHp (Actor|GetComponentbyClass _asplayable_character "/Script/BossFight.StatComponent")) 0))
        (Class|PlayableCharacter|TakeDamage _asplayable_character "Hit" (Variables|/Script/BossFight.StatComponent|GetDamage (Variables|Default|GetStatComponent)) self)))))

(event Custom|ATK_01
  (params (Target :type Actor%20Object%20Reference))
  ;[0.4522 0.4522 0.4522] ATK_01
  (Utilities|FlowControl|Sequence
    (:then_0
      (Utilities|IsValid Target
        (:Is%20Valid
          (bind _returnvalue (Transformation|SetActorRotation (Math|Rotator|MakeRotator 0.0 0.0 (.yaw (Math|Rotator|FindLookatRotation (Transformation|GetActorLocation) (Transformation|GetActorLocation Target)))))))))
    (:then_1
      (Animation|PlayAnimMontage (Utilities|Array|Get(acopy) (Variables|Default|GetAttackArray) (Math|Random|RandomIntegerinRange 0 1)) 1.0 "None"))))

(event Custom|OnGameStarted_Event
  (Variables|Default|SetbGameStarted false))

(event EventBeginPlay
  (Class|StatComponent|InitStat (Variables|Default|GetStatComponent) "Boss")
  (bind _asmanager (Utilities|Casting|CastToManager (Game|GetGameInstance)))
  (EventDispatchers|AssignOnGameStarted _asmanager (delegate Custom|OnGameStarted_Event)))

(event EventTick
  (params (DeltaSeconds :type Float%20%28single-precision%29))
  (bind _target (CallFunction|GetTarget))
  ;[0.3854 0.3854 0.3854] Overlap Set, Get and Clear Target
  (if (Variables|Default|GetbGameStarted)
    (if (Utilities|IsValid _target)
      (if (<= (Variables|/Script/BossFight.StatComponent|GetHp (Actor|GetComponentbyClass _target "/Script/BossFight.StatComponent")) 0)
        (CallFunction|SetTarget) ; 타겟의 체력이 0보다 적으면 타겟 해제
      ))))

(fn ConstructionScript)

(fn SetTarget
  (params (NewTarget :type Actor%20Object%20Reference))
  (AI|Components|Blackboard|SetValueasObject (AI|GetBlackboard (AI|GetAIController self)) (Utilities|Name|MakeLiteralName "Target") NewTarget))

(fn GetTarget
  (return (.AsActor (Utilities|Casting|CastToActor (AI|Components|Blackboard|GetValueasObject (AI|GetBlackboard (AI|GetAIController self)) (Utilities|Name|MakeLiteralName "Target"))))))

(fn ClearTarget
  (AI|Components|Blackboard|ClearValue (AI|GetBlackboard (AI|GetAIController self)) (Utilities|Name|MakeLiteralName "Target")))