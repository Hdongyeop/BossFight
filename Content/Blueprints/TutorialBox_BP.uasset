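; TutorialBox_BP is a trigger box that shows the Tutorial_WBP widget on screen while the player is inside it.
; A new widget is created and added to the viewport when a PlayableCharacter begins overlapping the collision component, and also when the Manager game instance signals game start.
; Any end overlap, regardless of actor, removes the most recently stored widget.
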(event OnComponentBeginOverlap(CollisionComponent)
  (params (OverlappedComponent :type Primitive%20Component%20Object%20Reference) (OtherActor :type Actor%20Object%20Reference) (OtherComp :type Primitive%20Component%20Object%20Reference) (OtherBodyIndex :type Integer) (bFromSweep :type Boolean) (SweepResult :type Hit%20Result%20Structure%20%28by%20ref%29))
  (Utilities|Casting|CastToPlayableCharacter OtherActor)
  (bind _returnvalue (UserInterface|CreateWidget "/Game/UI/Tutorial_WBP.Tutorial_WBP_C" (Game|GetPlayerController 0)))
  (UserInterface|Viewport|AddtoViewport _returnvalue 0)
  (Variables|Default|SetTutorialWidget _returnvalue))

(event OnComponentEndOverlap(CollisionComponent)
  (params (OverlappedComponent :type Primitive%20Component%20Object%20Reference) (OtherActor :type Actor%20Object%20Reference) (OtherComp :type Primitive%20Component%20Object%20Reference) (OtherBodyIndex :type Integer))
  (bind _tutorialwidget (Variables|Default|GetTutorialWidget))
  (Utilities|IsValid _tutorialwidget
    (:Is%20Valid
      (Widget|RemovefromParent _tutorialwidget))))

(event Custom|OnGameStarted_Event
  (bind _returnvalue (UserInterface|CreateWidget "/Game/UI/Tutorial_WBP.Tutorial_WBP_C" (Game|GetPlayerController 0)))
  (UserInterface|Viewport|AddtoViewport _returnvalue 0)
  (Variables|Default|SetTutorialWidget _returnvalue))

(event EventBeginPlay
  (bind _asmanager (Utilities|Casting|CastToManager (Game|GetGameInstance)))
  (EventDispatchers|AssignOnGameStarted _asmanager (delegate Custom|OnGameStarted_Event)))

(fn ConstructionScript)